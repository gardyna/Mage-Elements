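; Combat utility Blueprint function library that applies knockback to a hit component, whether a physics object or a character.
; Physics-simulating components are woken and receive a mass-scaled impulse at the impact location, so the velocity change does not depend on weight.
; Otherwise the owning Character stops moving and is launched by the multiplied impulse plus a fixed upward boost, overriding its velocity; other owners are ignored.
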(fn `ApplyKnockback`
  (params (`Target Component` :type "PrimitiveComponent Object Reference") (`Impulse Vector` :type "Vector Structure") (`Impact Location` :type "Vector Structure"))
  (locals (Component :type "PrimitiveComponent Object Reference") (impulse :type "Vector Structure") (Location :type "Vector Structure") (`Character Launch Multiplier` :type "Float (double-precision)" :default 5.0))
  (bind _component (`local.Component`))
  (set `local.impulse` `Impulse Vector`)
  (set `local.Location` `Impact Location`)
  (set `local.Component` `Target Component`)
  (if (`SceneComponent.IsSimulatingPhysics` `Target Component` "None")
    ; As object
    (`PrimitiveComponent.WakeRigidBody` _component "None")
    (`PrimitiveComponent.AddImpulseAtLocation` _component (* (`PrimitiveComponent.GetMass` (`local.Component`)) (`local.impulse`)) (`local.Location`) "None")
    (else
      (bind _ascharacter (cast `Character` (`ActorComponent.GetOwner` `Target Component`)))
      ; As Character
      (`MovementComponent.StopMovementImmediately` (`Character.CharacterMovement` _ascharacter))
      (`Character.LaunchCharacter` _ascharacter (+ (* (`local.impulse`) (`local.Character Launch Multiplier`)) (0.0 0.0 200.0)) true true))))