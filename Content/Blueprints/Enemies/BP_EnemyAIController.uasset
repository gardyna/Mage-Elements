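; Enemy AI controller that runs the enemy behavior tree and feeds it the player as a target when seen.
; On possess it starts BT_Enemy and prints the result.
; On each perception update it checks whether sight currently perceives the player character, then sets or clears the blackboard target actor key, with debug prints left in.
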(event `self.ReceivePossess`
  (params (PossessedPawn :type "Pawn Object Reference"))
  (bind _returnvalue (`self.RunBehaviorTree` "/Game/Blueprints/Enemies/BT_Enemy.BT_Enemy"))
  (`KismetSystemLibrary.PrintString` (`KismetStringLibrary.Conv_BoolToString` _returnvalue) true true (struct :`G` 1.0 :`B` 0.059202 :`A` 1.0)))

(event `self.AIPerception.OnPerceptionUpdated`
  (params (UpdatedActors :type "Array of Actor Object Reference (by ref)"))
  (bind _returnvalue (`GameplayStatics.GetPlayerCharacter` 0))
  (bind _returnvalue_2 (`AIBlueprintHelperLibrary.GetBlackboard` null))
  (bind _actortargetname (`self.ActorTargetName`))
  ; Visibility (look for player)
  (`KismetSystemLibrary.PrintString` "Perception update")
  (if (`KismetArrayLibrary.Array_Contains` (`AIPerceptionComponent.GetCurrentlyPerceivedActors` (`self.AIPerception`) "/Script/AIModule.AISense_Sight") _returnvalue)
    (`BlackboardComponent.SetValueAsObject` _returnvalue_2 _actortargetname _returnvalue)
    (else
      (`BlackboardComponent.SetValueAsObject` _returnvalue_2 _actortargetname null))))

(fn `UserConstructionScript`)