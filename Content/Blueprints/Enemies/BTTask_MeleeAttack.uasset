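; Behavior tree task that makes an enemy deal melee damage to the target actor stored on its blackboard.
; It builds a GE_EnemyDamage effect spec with a fixed Set By Caller magnitude on the Data.Damage tag and applies it from the pawn's ability system to the target's.
; The damage lands immediately with no range check or animation, and the task fails only when the blackboard target is not a valid Actor.
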(event `self.ReceiveExecuteAI`
  (params (OwnerController :type "AIController Object Reference") (ControlledPawn :type "Pawn Object Reference"))
  ; Get ability systems
  (bind _asactor (cast `Actor` (`BlackboardComponent.GetValueAsObject` (`AIBlueprintHelperLibrary.GetBlackboard` OwnerController) (`self.TargetActor`)))
    (:`then`
      (set `self.TargetAbilitySystem` (`AbilitySystemBlueprintLibrary.GetAbilitySystemComponent` _asactor))
      (set `self.SelfAbilitySystem` (`AbilitySystemBlueprintLibrary.GetAbilitySystemComponent` ControlledPawn))
      ; Create attack effect
      (`KismetSystemLibrary.PrintString` "Attacking")
      (bind _returnvalue (`AbilitySystemBlueprintLibrary.MakeSpecHandleByClass` "/Game/Blueprints/Enemies/GE_EnemyDamage.GE_EnemyDamage_C"))
      (bind _returnvalue_2 (`AbilitySystemBlueprintLibrary.AssignTagSetByCallerMagnitude` _returnvalue (struct :`TagName` "Data.Damage") 25.0))
      (`AbilitySystemComponent.BP_ApplyGameplayEffectSpecToTarget` (`self.SelfAbilitySystem`) _returnvalue_2 (`self.TargetAbilitySystem`))
      (`self.FinishExecute` true))
    (:`CastFailed`
      (`self.FinishExecute` false))))