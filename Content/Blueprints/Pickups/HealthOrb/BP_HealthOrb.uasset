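; BP_HealthOrb is a timed health pickup that heals the first-person player character on touch.
; On BeginPlay it scales its sphere mesh by heal amount and starts a lifetime timer that destroys it.
; On overlap it compares two Ability System attributes, then applies GE_HealthRestore with HealAmount as a Data.Heal SetByCaller magnitude, plays a ping and destroys itself.
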(event `self.ReceiveBeginPlay`
  (bind _spheremesh (`self.SphereMesh`))
  ; Start fadeOut timer
  (`KismetSystemLibrary.K2_SetTimerDelegate` (delegate `Expire`) (`self.Lifetime`))
  ; Size relative to heal amount
  (`SceneComponent.SetRelativeScale3D` _spheremesh (`KismetMathLibrary.Conv_DoubleToVector` (`KismetMathLibrary.MapRangeClamped` (`self.HealAmount`) 10.0 50.0 0.75 1.5)))
  (`KismetSystemLibrary.PrintString` (`KismetStringLibrary.Conv_VectorToString` (`SceneComponent.K2_GetComponentScale` _spheremesh))))

(event `Expire`
  (`self.K2_DestroyActor`))

(event `self.SphereCollision.OnComponentBeginOverlap`
  (params (OverlappedComponent :type "PrimitiveComponent Object Reference") (OtherActor :type "Actor Object Reference") (OtherComp :type "PrimitiveComponent Object Reference") (OtherBodyIndex :type Integer) (bFromSweep :type Boolean) (SweepResult :type "HitResult Structure (by ref)"))
  (bind _asbp_first_person_character (cast `/Game/FirstPerson/Blueprints/BP_FirstPersonCharacter` OtherActor))
  (bind _returnvalue (`AbilitySystemBlueprintLibrary.GetAbilitySystemComponent` _asbp_first_person_character))
  (bind (_bsuccessfullyfoundattribute _returnvalue_2) (`AbilitySystemBlueprintLibrary.GetFloatAttributeFromAbilitySystemComponent` _returnvalue (struct :`AttributeName` "Health" :`Attribute` "/Script/MageGame.MageAttributeSet:Health" :`AttributeOwner` "/Script/CoreUObject.Class'/Script/MageGame.MageAttributeSet'")))
  (bind (_bsuccessfullyfoundattribute_2 _returnvalue_3) (`AbilitySystemBlueprintLibrary.GetFloatAttributeFromAbilitySystemComponent` _returnvalue (struct :`AttributeName` "MaxHealth" :`Attribute` "/Script/MageGame.MageAttributeSet:MaxHealth" :`AttributeOwner` "/Script/CoreUObject.Class'/Script/MageGame.MageAttributeSet'")))
  (if (and (and _bsuccessfullyfoundattribute _bsuccessfullyfoundattribute_2) (< _returnvalue_2 _returnvalue_3))
    (bind _returnvalue_4 (`AbilitySystemBlueprintLibrary.MakeSpecHandleByClass` "/Game/Blueprints/Pickups/HealthOrb/GE_HealthRestore.GE_HealthRestore_C"))
    (bind _returnvalue_5 (`AbilitySystemBlueprintLibrary.AssignTagSetByCallerMagnitude` _returnvalue_4 (struct :`TagName` "Data.Heal") (`self.HealAmount`)))
    (`AbilitySystemComponent.BP_ApplyGameplayEffectSpecToSelf` _returnvalue _returnvalue_5)
    (`GameplayStatics.PlaySoundAtLocation` "/Engine/EngineSounds/1kSineTonePing.1kSineTonePing" (`self.K2_GetActorLocation`) (struct) 1.0 1.0 0.0 null null null null)
    (`self.K2_DestroyActor`)))

(fn `UserConstructionScript`)