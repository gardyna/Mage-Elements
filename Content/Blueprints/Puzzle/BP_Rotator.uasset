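; BP_Rotator is a puzzle actor that rotates through a RotatingMovement component, switched on and off by a linked interactable.
; On BeginPlay it copies its RotationRate to the component and, if ControllingInteractable is valid, binds to its trigger-toggled event and deactivates rotation.
; Each toggle then activates or deactivates the movement without resetting it.
; Without a valid interactable, the Blueprint leaves the component's active state untouched.
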(event `self.ReceiveBeginPlay`
  (bind _controllinginteractable (`self.ControllingInteractable`))
  (set `RotatingMovementComponent.RotationRate` (`self.RotationRate`) (`self.RotatingMovement`))
  (if (`KismetSystemLibrary.IsValid` _controllinginteractable)
    (add `/Game/Blueprints/Puzzle/BP_PuzzleTrigger.OnTriggerToggled` _controllinginteractable (delegate `TriggerToggled`))
    (`ActorComponent.SetActive` (`self.RotatingMovement`) false false :!label _label)))

(event `TriggerToggled`
  (params (bIsOn :type Boolean))
  (if bIsOn
    (`ActorComponent.SetActive` (`self.RotatingMovement`) true false)
    (else
      (goto _label))))

(fn `UserConstructionScript`)