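; BP_TogglePhysics is a puzzle actor whose Cube switches physics simulation on or off in response to a linked interactable.
; On BeginPlay it binds to the trigger toggle event of ControllingInteractable, if that reference is valid.
; Simulation is the inverse of the trigger state: on disables it and prints a message, while off zeroes linear and angular velocity, then enables it.
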(event `self.ReceiveBeginPlay`
  (bind _controllinginteractable (`self.ControllingInteractable`))
  (if (`KismetSystemLibrary.IsValid` _controllinginteractable)
    (add `/Game/Blueprints/Puzzle/BP_PuzzleTrigger.OnTriggerToggled` _controllinginteractable (delegate `OnTriggerToggled`))))

(event `OnTriggerToggled`
  (params (bIsOn :type Boolean))
  (bind _returnvalue (not bIsOn))
  (bind _cube (`self.Cube`))
  (if _returnvalue
    (`PrimitiveComponent.SetPhysicsAngularVelocityInDegrees` _cube (0.0 0.0 0.0) false "None")
    (`PrimitiveComponent.SetPhysicsLinearVelocity` _cube (0.0 0.0 0.0) false "None")
    (else
      (`KismetSystemLibrary.PrintString` "Physics off")))
  (`PrimitiveComponent.SetSimulatePhysics` _cube _returnvalue))

(fn `UserConstructionScript`)