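; Puzzle fire spout that plays a Niagara fire stream and ignites actors in a cone ahead of it.
; It starts spouting on BeginPlay, and an optional controlling interactable can toggle the stream and its looping timer.
; Each timer tick fires five sphere traces in a cross spanning the cone, sending IgniteMessage to every hit actor.
; Persistent trace drawing and a debug print are left enabled.
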(event `self.ReceiveBeginPlay`
  (bind _controllinginteractable (`self.ControllingInteractable`))
  (if (`KismetSystemLibrary.IsValid` _controllinginteractable)
    (add `/Game/Blueprints/Puzzle/BP_PuzzleTrigger.OnTriggerToggled` _controllinginteractable (delegate `OnTriggerToggled_Event`)))
  (bind _returnvalue (`KismetSystemLibrary.K2_SetTimerDelegate` (delegate `PeriodicIgnite`) 0.5 true :!label _label))
  (set `self.SpoutTimerHandle` _returnvalue)
  (`ActorComponent.Activate` (`self.NS_FireStream`) false))

(event `OnTriggerToggled_Event`
  (params (bIsOn :type Boolean))
  (bind _output_get (set `self.bIsSpouting` bIsOn))
  (if _output_get
    (goto _label)
    (else
      (`KismetSystemLibrary.K2_ClearAndInvalidateTimerHandle` (`self.SpoutTimerHandle`))
      (`ActorComponent.Deactivate` (`self.NS_FireStream`)))))

(event `PeriodicIgnite`
  (bind _conehalfangle (`self.ConeHalfAngle`))
  (bind _returnvalue (* _conehalfangle -1.0))
  (`|ExecutionSequence`
    (:`then_0`
      (`self.FireRay` 0.0))
    (:`then_1`
      (`self.FireRay` 0.0 _conehalfangle))
    (:`then_2`
      (`self.FireRay` 0.0 _returnvalue))
    (:`then_3`
      (`self.FireRay` _conehalfangle))
    (:`then_4`
      (`self.FireRay` _returnvalue))))

(fn `FireRay`
  (params (PitchOffset :type "Float (double-precision)") (YawOffset :type "Float (double-precision)"))
  (locals (`Forward Vector` :type "Vector Structure") (Start :type "Vector Structure" :default (0.0 0.0 0.0)) (End :type "Vector Structure"))
  (bind _fire_cone_folder (`self.Fire cone folder`))
  (bind _output_get (set `local.Start` (`SceneComponent.K2_GetComponentLocation` _fire_cone_folder)))
  (bind _outhits (`KismetSystemLibrary.SphereTraceMulti` :`Start` _output_get :`End` (+ _output_get (* (`KismetMathLibrary.GetForwardVector` (`KismetMathLibrary.ComposeRotators` (`KismetMathLibrary.Conv_VectorToRotator` (`SceneComponent.GetForwardVector` _fire_cone_folder)) (`KismetMathLibrary.MakeRotator` 0.0 PitchOffset YawOffset))) (`self.Reach`))) :`Radius` 50.0 :`TraceChannel` "TraceTypeQuery4" :`DrawDebugType` "Persistent"))
  (for _array_element _outhits
    (message `/Game/Blueprints/Interaction/BPI_Ignitable.Ignite` (`.HitActor` (`GameplayStatics.BreakHitResult` _array_element)) 0.0)
    (`KismetSystemLibrary.PrintString` "Set Fire")))

(fn `UserConstructionScript`)