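; BP_RotatingPaddle is a puzzle actor that builds a paddle at the top of a pole, offset from a hinge.
; The construction script sizes the pole and paddle from PoleHeight and PaddleLength, then positions the hinge at the pole top with the paddle extending outward.
; SpinDamping sets the paddle's angular damping.
; The event graph has no active logic, so any rotation is left to the components.
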(fn `UserConstructionScript`
  (bind _paddle (`self.Paddle`))
  (bind _paddlelength (`self.PaddleLength`))
  (bind _pole (`self.Pole`))
  (bind _poleheight (`self.PoleHeight`))
  (`SceneComponent.SetRelativeScale3D` _pole (`KismetMathLibrary.MakeVector` 0.2 0.2 (/ _poleheight 100.0)))
  (`SceneComponent.K2_SetRelativeLocation` _pole (`KismetMathLibrary.MakeVector` 0.0 0.0 (/ _poleheight 2.0)) false false)
  (`SceneComponent.K2_SetRelativeLocation` (`self.Hinge`) (`KismetMathLibrary.MakeVector` 0.0 0.0 (`self.PoleHeight`)) false false)
  (`SceneComponent.SetRelativeScale3D` _paddle (`KismetMathLibrary.MakeVector` (/ _paddlelength 100.0) 0.3 1.0))
  (`SceneComponent.K2_SetRelativeLocation` _paddle (`KismetMathLibrary.MakeVector` (/ _paddlelength 2.0) 0.0 (`self.PoleHeight`)) false false)
  (`PrimitiveComponent.SetAngularDamping` (`self.Paddle`) (`self.SpinDamping`)))