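; Fire Blast gameplay ability: a cone-shaped burst of fire from the avatar's eyes that also launches the caster backward.
; On commit it applies cost, cooldown and mana-regen delay, then filters a sphere overlap by view cone and line of sight.
; Hit targets receive distance-scaled SetByCaller damage and knockback, plus burning and an ignite message.
; The gameplay cue and self-knockback run even if commit fails; debug traces and prints remain.
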(event `self.K2_ActivateAbility`
  (bind _returnvalue (`self.GetAvatarActorFromActorInfo`))
  (bind (_outlocation _outrotation) (`Actor.GetActorEyesViewPoint` (`self.GetAvatarActorFromActorInfo`)))
  (bind (_outlocation_2 _outrotation_2) (`Actor.GetActorEyesViewPoint` _returnvalue))
  (bind _array (`|MakeArray` (`self.GetAvatarActorFromActorInfo`)))
  (`GameplayCueFunctionLibrary.ExecuteGameplayCueOnActor` _returnvalue (struct :`TagName` "GameplayCue.Spell.FireBlast") (`AbilitySystemBlueprintLibrary.MakeGameplayCueParameters` 0.0 0.0 (struct) (struct) (struct) (struct) (struct) (- _outlocation_2 (0.0 0.0 20.0)) (`KismetMathLibrary.GetForwardVector` _outrotation_2)))
  (`|ExecutionSequence`
    (:`then_0`
      (bind _returnvalue_2 (`self.K2_CommitAbility`))
      (if _returnvalue_2
        (`self.BP_ApplyGameplayEffectToOwner` "/Game/Blueprints/Spells/FireBlast/GE_Cost_FireBlast.GE_Cost_FireBlast_C")
        (`self.BP_ApplyGameplayEffectToOwner` "/Game/Blueprints/Spells/FireBlast/GE_Cooldown_FireBlast.GE_Cooldown_FireBlast_C")
        (`self.BP_ApplyGameplayEffectToOwner` "/Game/Blueprints/Abilities/GE_ManaRegenDelay.GE_ManaRegenDelay_C")
        (bind _outactors (`KismetSystemLibrary.SphereOverlapActors` _outlocation (`self.BlastRange`) (`|MakeArray` "ObjectTypeQuery4" "ObjectTypeQuery3" "ObjectTypeQuery2" :!type "EObjectTypeQuery Enum") null _array))
        (for _array_element _outactors
          (bind (_is_in_cone _dot_product _target_location) (`self.Is Actor In View Cone` _array_element _outlocation _outrotation))
          (if _is_in_cone
            ; Wall check
            (bind (_outhit _returnvalue_3) (`KismetSystemLibrary.LineTraceSingle` _outlocation _target_location "TraceTypeQuery1" false _array "ForDuration" false))
            (if (and (== (`.HitActor` (`GameplayStatics.BreakHitResult` _outhit)) _array_element) _returnvalue_3)
              (`self.Apply Fire Blast` (`.HitActor` (`GameplayStatics.BreakHitResult` _outhit)) (`.HitComponent` (`GameplayStatics.BreakHitResult` _outhit)) (`.ImpactPoint` (`GameplayStatics.BreakHitResult` _outhit)) _outlocation (`.Distance` (`GameplayStatics.BreakHitResult` _outhit)))
              (else
                (`KismetSystemLibrary.PrintString` "blocked")))
            (else
              (`KismetSystemLibrary.PrintString` "Not in cone")))))
      (`self.K2_EndAbility`))
    (:`then_1`
      (`self.SelfKnockback`))))

(fn `Apply Fire Blast`
  (params (`Target Actor` :type "Actor Object Reference") (`Target Component` :type "PrimitiveComponent Object Reference") (`impact point` :type "Vector Structure") (`From Location` :type "Vector Structure") (Distance :type "Float (double-precision)"))
  (locals (From :type "Vector Structure") (To :type "Vector Structure") (TargetActor :type "Actor Object Reference") (TargetComponent :type "PrimitiveComponent Object Reference") (ImpactPoint :type "Vector Structure") (ImpactDistance :type "Float (double-precision)"))
  (bind _returnvalue (`AbilitySystemBlueprintLibrary.GetAbilitySystemComponent` (`local.TargetActor`)))
  (set `local.ImpactDistance` Distance)
  (set `local.TargetActor` `Target Actor`)
  (set `local.TargetComponent` `Target Component`)
  (set `local.From` `From Location`)
  (set `local.To` `impact point`)
  (set `local.ImpactPoint` `impact point`)
  ; Gameplay effects
  (if (`KismetSystemLibrary.IsValid` _returnvalue)
    (bind _returnvalue_2 (`AbilitySystemBlueprintLibrary.AssignTagSetByCallerMagnitude` (`self.MakeOutgoingGameplayEffectSpec` "/Game/Blueprints/Spells/FireBlast/GE_FireDamage.GE_FireDamage_C") (struct :`TagName` "Data.Damage") (`KismetMathLibrary.MapRangeClamped` (`local.ImpactDistance`) 0.0 (`self.BlastRange`) (`self.MaxDamage`) (`self.MinDamage`))))
    (`AbilitySystemComponent.BP_ApplyGameplayEffectSpecToTarget` _returnvalue _returnvalue_2 null)
    (`AbilitySystemComponent.BP_ApplyGameplayEffectSpecToTarget` _returnvalue (`self.MakeOutgoingGameplayEffectSpec` "/Game/Blueprints/Spells/FireBlast/GE_Burning.GE_Burning_C") null))
  ; Apply impulse
  (`/Game/Blueprints/Common/BPFL_CombatUtils.ApplyKnockback` (`local.TargetComponent`) (* (`KismetMathLibrary.MapRangeClamped` (`local.ImpactDistance`) 0.0 (`self.BlastRange`) (`self.MaxForce`) (`self.MinForce`)) (`KismetMathLibrary.GetDirectionUnitVector` (`local.From`) (`local.To`))) (`local.ImpactPoint`))
  (message `/Game/Blueprints/Interaction/BPI_Ignitable.Ignite` (`local.TargetActor`) (`KismetMathLibrary.MapRangeClamped` (`local.ImpactDistance`) 0.0 (`self.BlastRange`) (`self.MaxDamage`) (`self.MinDamage`))))

(fn `Is Actor In View Cone`
  (params (`Actor To Check` :type "Actor Object Reference") (`Eye Location` :type "Vector Structure") (`Eye Rotation` :type "Rotator Structure"))
  (returns (`Is in cone` :type Boolean) (`Dot product` :type "Float (double-precision)") (`Target Location` :type "Vector Structure"))
  (bind _returnvalue (`Actor.K2_GetActorLocation` `Actor To Check`))
  (bind _returnvalue_2 (`KismetMathLibrary.Dot_VectorVector` (`KismetMathLibrary.GetDirectionUnitVector` `Eye Location` _returnvalue) (`KismetMathLibrary.GetForwardVector` `Eye Rotation`)))
  (return (< (`KismetMathLibrary.DegCos` (`self.ConeHalfAngle`)) _returnvalue_2) _returnvalue_2 _returnvalue))

(fn `SelfKnockback`
  (bind _returnvalue (`self.GetAvatarActorFromActorInfo`))
  (bind _ascharacter (cast `Character` _returnvalue))
  (`Character.LaunchCharacter` _ascharacter (* (`KismetMathLibrary.GetForwardVector` (`.OutRotation` (`Actor.GetActorEyesViewPoint` _returnvalue))) (* (`self.SelfKnockbackStrength`) -1.0)) true true))