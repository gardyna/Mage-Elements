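; Arcane bolt spell projectile that damages what it hits, shoves physics objects and then destroys itself.
; Its collision sphere ignores the owning actor when moving and handles the hit event.
; ApplySpellImpulse pushes simulating components at the impact point along the sphere's forward vector, scaling ForceAmount by mass so objects react alike regardless of weight, and prints debug strings.
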(event `self.ReceiveBeginPlay`
  (`PrimitiveComponent.IgnoreActorWhenMoving` (`self.SphereCollision`) (`self.GetOwner`) true))

(event `self.SphereCollision.OnComponentHit`
  (params (HitComponent :type "PrimitiveComponent Object Reference") (OtherActor :type "Actor Object Reference") (OtherComp :type "PrimitiveComponent Object Reference") (NormalImpulse :type "Vector Structure") (Hit :type "HitResult Structure (by ref)"))
  (if (`SceneComponent.IsSimulatingPhysics` OtherComp "None")
    (`self.ApplySpellImpulse` OtherComp (`self.ForceAmount`) (`.ImpactPoint` (`GameplayStatics.BreakHitResult` Hit))))
  ; Deal Damage. Other may be dead after this point
  (`GameplayStatics.ApplyDamage` OtherActor (`KismetMathLibrary.Conv_IntToDouble` (`self.DamageAmount`)))
  (`self.K2_DestroyActor`))

(fn `ApplySpellImpulse`
  (params (TargetActor :type "PrimitiveComponent Object Reference") (ImpulseStrength :type "Float (double-precision)") (HitLocation :type "Vector Structure"))
  (bind _returnvalue (* (`KismetMathLibrary.Normal` (`SceneComponent.GetForwardVector` (`self.SphereCollision`))) (`self.ForceAmount`)))
  (if (`SceneComponent.IsSimulatingPhysics` TargetActor "None")
    (`KismetSystemLibrary.PrintString` (`KismetStringLibrary.Conv_VectorToString` _returnvalue))
    (`PrimitiveComponent.AddImpulseAtLocation` TargetActor (* _returnvalue (`PrimitiveComponent.GetMass` TargetActor)) HitLocation "None")
    (else
      (`KismetSystemLibrary.PrintString` "No physics"))))

(fn `UserConstructionScript`)