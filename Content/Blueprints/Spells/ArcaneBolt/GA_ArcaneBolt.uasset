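; Gameplay Ability that casts the Arcane Bolt spell for the first-person character.
; On activation it spawns BP_ArcaneBolt at the character's SpellSpawnPoint and sets mutual move-ignore between bolt and caster to prevent self-collision.
; It then applies cooldown and cost Gameplay Effects directly, without CommitAbility, and ends immediately.
; If the avatar cast fails, it ends without spawning or applying effects.
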(event `self.K2_ActivateAbility`
  (bind _asbp_first_person_character (cast `/Game/FirstPerson/Blueprints/BP_FirstPersonCharacter` (`self.GetAvatarActorFromActorInfo`))
    (:`then`
      (bind _returnvalue (`|SpawnActorFromClass` "/Game/Blueprints/Spells/ArcaneBolt/BP_ArcaneBolt.BP_ArcaneBolt_C" (`SceneComponent.K2_GetComponentToWorld` (`/Game/FirstPerson/Blueprints/BP_FirstPersonCharacter.SpellSpawnPoint` _asbp_first_person_character)) "Undefined" "MultiplyWithRoot" _asbp_first_person_character null))
      ; Two Way ignore between bolt and caster
      (`PrimitiveComponent.IgnoreActorWhenMoving` (`Character.CapsuleComponent` _asbp_first_person_character) _returnvalue true)
      (`PrimitiveComponent.IgnoreActorWhenMoving` (`/Game/Blueprints/Spells/ArcaneBolt/BP_ArcaneBolt.SphereCollision` _returnvalue) _asbp_first_person_character true)
      (`self.BP_ApplyGameplayEffectToOwner` "/Game/Blueprints/Spells/ArcaneBolt/GE_Cooldown_ArcaneBolt.GE_Cooldown_ArcaneBolt_C")
      (`self.BP_ApplyGameplayEffectToOwner` "/Game/Blueprints/Spells/ArcaneBolt/GE_Cost_ArcaneBolt.GE_Cost_ArcaneBolt_C")
      (`self.K2_EndAbility`))
    (:`CastFailed`
      (`self.K2_EndAbility`))))