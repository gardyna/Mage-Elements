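; Arcane bolt spell actor that knocks back and damages what it hits, ignoring its owner while moving.
; On hit it applies knockback along the collision sphere's forward vector, then destroys itself.
; If the target has an Ability System Component, the owner's ASC applies GE_ArcaneDamage to it, passing damage through SetByCaller tag Data.Damage.
; ApplySpellImpulse, not called here, prints its impulse but multiplies it by zero before applying knockback.
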(event `self.ReceiveBeginPlay`
  (`PrimitiveComponent.IgnoreActorWhenMoving` (`self.SphereCollision`) (`self.GetOwner`) true))

(event `self.SphereCollision.OnComponentHit`
  (params (HitComponent :type "PrimitiveComponent Object Reference") (OtherActor :type "Actor Object Reference") (OtherComp :type "PrimitiveComponent Object Reference") (NormalImpulse :type "Vector Structure") (Hit :type "HitResult Structure (by ref)"))
  (bind _returnvalue (`AbilitySystemBlueprintLibrary.GetAbilitySystemComponent` OtherActor))
  (`/Game/Blueprints/Common/BPFL_CombatUtils.ApplyKnockback` OtherComp (* (`KismetMathLibrary.Normal` (`SceneComponent.GetForwardVector` (`self.SphereCollision`))) (`self.ForceAmount`)) (`.ImpactPoint` (`GameplayStatics.BreakHitResult` Hit)))
  (if (and (`KismetSystemLibrary.IsValid` (`self.GetOwner`)) (`KismetSystemLibrary.IsValid` _returnvalue))
    (bind _returnvalue_2 (`AbilitySystemBlueprintLibrary.MakeSpecHandleByClass` "/Game/Blueprints/Spells/ArcaneBolt/GE_ArcaneDamage.GE_ArcaneDamage_C"))
    (bind _returnvalue_3 (`AbilitySystemBlueprintLibrary.AssignTagSetByCallerMagnitude` _returnvalue_2 (struct :`TagName` "Data.Damage") (`self.DamageAmount`)))
    (`AbilitySystemComponent.BP_ApplyGameplayEffectSpecToTarget` (`AbilitySystemBlueprintLibrary.GetAbilitySystemComponent` (`self.GetOwner`)) _returnvalue_3 _returnvalue)
    (`self.K2_DestroyActor`)
    (else
      (`self.K2_DestroyActor`))))

(fn `ApplySpellImpulse`
  (params (TargetActor :type "PrimitiveComponent Object Reference") (ImpulseStrength :type "Float (double-precision)") (HitLocation :type "Vector Structure"))
  (bind _returnvalue (* (`KismetMathLibrary.Normal` (`SceneComponent.GetForwardVector` (`self.SphereCollision`))) ImpulseStrength))
  (`KismetSystemLibrary.PrintString` (`KismetStringLibrary.Conv_VectorToString` _returnvalue))
  (`/Game/Blueprints/Common/BPFL_CombatUtils.ApplyKnockback` TargetActor (* _returnvalue (0.0 0.0 0.0)) HitLocation))

(fn `UserConstructionScript`)