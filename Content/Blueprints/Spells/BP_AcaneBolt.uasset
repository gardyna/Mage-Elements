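; BP_AcaneBolt is a spell bolt that damages what it hits, pushes physics objects and then destroys itself.
; Its collision sphere ignores the owner when moving from BeginPlay, and each hit applies DamageAmount to the other actor.
; ApplySpellImpulse pushes simulating components along the sphere's forward vector, scaled by ForceAmount rather than its ImpulseStrength input, with debug prints.
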(event `self.ReceiveBeginPlay`
  (`PrimitiveComponent.IgnoreActorWhenMoving` (`self.SphereCollision`) (`self.GetOwner`) true))

(event `self.SphereCollision.OnComponentHit`
  (params (HitComponent :type "PrimitiveComponent Object Reference") (OtherActor :type "Actor Object Reference") (OtherComp :type "PrimitiveComponent Object Reference") (NormalImpulse :type "Vector Structure") (Hit :type "HitResult Structure (by ref)"))
  (`GameplayStatics.ApplyDamage` OtherActor (`KismetMathLibrary.Conv_IntToDouble` (`self.DamageAmount`)))
  (if (`SceneComponent.IsSimulatingPhysics` OtherComp "None")
    (`self.ApplySpellImpulse` OtherComp (`self.ForceAmount`)))
  (`self.K2_DestroyActor`))

(fn `ApplySpellImpulse`
  (params (TargetActor :type "PrimitiveComponent Object Reference") (ImpulseStrength :type "Float (double-precision)"))
  (bind _returnvalue (* (`KismetMathLibrary.Normal` (`SceneComponent.GetForwardVector` (`self.SphereCollision`))) (`self.ForceAmount`)))
  (if (`SceneComponent.IsSimulatingPhysics` TargetActor "None")
    (`KismetSystemLibrary.PrintString` (`KismetStringLibrary.Conv_VectorToString` _returnvalue))
    (`PrimitiveComponent.AddImpulse` TargetActor _returnvalue "None" false)
    (else
      (`KismetSystemLibrary.PrintString` "No physics"))))

(fn `UserConstructionScript`)