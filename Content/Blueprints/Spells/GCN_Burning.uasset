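; Gameplay cue notify that shows a burning visual effect on its target.
; WhileActive attaches a Niagara system to the target's skeletal mesh component, or falls back to a static-mesh variant on its static mesh component when none exists.
; It stores the spawned system so OnRemove can deactivate it when the cue ends.
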(event `self.K2_HandleGameplayCue`
  (params (MyTarget :type "Actor Object Reference") (EventType :type "EGameplayCueEvent Enum" :default "OnActive") (Parameters :type "GameplayCueParameters Structure (by ref)")))

(fn `OnRemove`
  (params (MyTarget :type "Actor Object Reference") (Parameters :type "GameplayCueParameters Structure (by ref)"))
  (returns (ReturnValue :type Boolean))
  (bind _burningeffect (`self.BurningEffect`))
  (if (`KismetSystemLibrary.IsValid` _burningeffect)
    (`ActorComponent.Deactivate` _burningeffect))
  (return false))

(fn `UserConstructionScript`)

(fn `WhileActive`
  (params (MyTarget :type "Actor Object Reference") (Parameters :type "GameplayCueParameters Structure (by ref)"))
  (returns (ReturnValue :type Boolean))
  (bind _returnvalue (`self.GetComponentByClass` MyTarget "/Script/Engine.SkeletalMeshComponent"))
  (if (`KismetSystemLibrary.IsValid` _returnvalue)
    (bind _returnvalue_2 (`NiagaraFunctionLibrary.SpawnSystemAttached` "/Game/Blueprints/Spells/NS_Burning.NS_Burning" _returnvalue "None" (0.0 0.0 0.0) (struct) "KeepRelativeOffset"))
    (set `self.BurningEffect` _returnvalue_2)
    (else
      (bind _returnvalue_3 (`NiagaraFunctionLibrary.SpawnSystemAttached` "/Game/Blueprints/Spells/NS_Burning_StaticMesh.NS_Burning_StaticMesh" (`self.GetComponentByClass` MyTarget "/Script/Engine.StaticMeshComponent") "None" (0.0 0.0 0.0) (struct) "KeepRelativeOffset"))
      (set `self.BurningEffect` _returnvalue_3)))
  (return false))