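; BP_PhysicsTarget is an environment actor with a Cube component that can be set on fire.
; Its Ignite event adds the Burning gameplay cue to the cube's owning actor, with no other logic in the graph.
; It implements SPUD save-system callbacks with default answers: default respawn mode, no name override, and no skipping of the object or its transform and velocity restore.
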(event `self.ReceiveBeginPlay`)

(event `/Game/Blueprints/Interaction/BPI_Ignitable.Ignite`
  (params (Intensity :type "Float (double-precision)"))
  (`GameplayCueFunctionLibrary.AddGameplayCueOnActor` (`ActorComponent.GetOwner` (`self.Cube`)) (struct :`TagName` "GameplayCue.Effect.Burning") (`AbilitySystemBlueprintLibrary.MakeGameplayCueParameters` 0.0)))

(fn `GetSpudRespawnMode`
  (returns (ReturnValue :type "ESpudRespawnMode Enum"))
  (return "Default"))

(fn `OverrideName`
  (returns (ReturnValue :type String))
  (return ""))

(fn `ShouldSkip`
  (returns (ReturnValue :type Boolean))
  (return false))

(fn `ShouldSkipRestoreTransform`
  (returns (ReturnValue :type Boolean))
  (return false))

(fn `ShouldSkipRestoreVelocity`
  (returns (ReturnValue :type Boolean))
  (return false))

(fn `UserConstructionScript`)